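; BP_RepairPart is a repair part from the tank's parts fabricator module, configured at runtime from its Name variable.
; On BeginPlay it prints Name, looks up that row in DT_RepairParts, then applies the row's mesh and enables physics simulation.
; It derives its RepairNeed by looping over ENUM_RepairNeed for the entry whose name matches the row's Name field.
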(event EventBeginPlay
  (bind _name (Variables|Default|GetName))
  (Development|PrintString (Utilities|String|ToString(Name) _name))
  (bind _returnvalue (Utilities|GetDataTableRow "/Game/CyberTanks/TankBase/Modules/PartsFabricator/RepairPart/DT_RepairParts.DT_RepairParts" _name)
    (:then
      (Components|StaticMesh|SetStaticMesh (Variables|Default|GetStaticMesh) (.Mesh (Utilities|Struct|BreakSTRUCT_RepairPart _returnvalue)))
      (Physics|SetSimulatePhysics (Variables|Default|GetStaticMesh) true)
      (bind _enumvalue (|ForEachENUM_RepairNeed)
        (:LoopBody
          (if (== (Utilities|Name|EnumtoName _enumvalue) (.Name (Utilities|Struct|BreakSTRUCT_RepairPart _returnvalue)))
            (Variables|Default|SetRepairNeed _enumvalue)))
        (:then)))))

(fn ConstructionScript)