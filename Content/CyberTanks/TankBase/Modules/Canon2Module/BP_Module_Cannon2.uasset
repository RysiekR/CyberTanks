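; BP_Module_Cannon2 is a cannon module Blueprint for a tank.
; BeginPlay runs the parent logic and binds to a move-triggered event, while the Interact input and AimEvent handlers are empty.
; Disconnected logic would shoot the cannon at an Energon energy cost when usable, and aim it from normalized, sensitivity-scaled input, but none of it currently runs.
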(event Custom|AimEvent
  (params (ActionValue :type Vector%202D%20Structure)))

(event Input|EnhancedActionEvents|EnhancedInputActionIA_Interact
  (params (ActionValue :type Boolean) (ElapsedSeconds :type Float%20%28double-precision%29) (TriggeredSeconds :type Float%20%28double-precision%29) (InputAction :type Input%20Action%20Object%20Reference :default "/Game/ThirdPerson/Input/Actions/IA_Interact.IA_Interact")))

(event EventBeginPlay
  (|CallParentFunction)
  (EventDispatchers|BindEventtoMoveTriggeredEvent (EventDispatchers|CreateEvent :!event Custom|AimEvent)))

(fn ConstructionScript
  (|CallParentFunction))