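; Tank shield module that wraps the vehicle in a sphere, toggled on and off by interaction and starting switched off.
; When usable, it destroys overlapping BP_Bullets not owned by a tank part, charging both their HP and energy damage to ACEnergon energy.
; ACEnergon zero-HP or zero-energy events drop the shield by disabling sphere visibility and overlap events.
; The sphere snaps to the owning vehicle's mesh shortly after BeginPlay.
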(event OnComponentBeginOverlap(Shield_Sphere)
  (params (OverlappedComponent :type Primitive%20Component%20Object%20Reference) (OtherActor :type Actor%20Object%20Reference) (OtherComp :type Primitive%20Component%20Object%20Reference) (OtherBodyIndex :type Integer) (bFromSweep :type Boolean) (SweepResult :type Hit%20Result%20Structure%20%28by%20ref%29))
  (bind _asbp_bullet (Utilities|Casting|CastToBP_Bullet OtherActor))
  (Class|KismetSystemLibrary|IsObjectOfSoftClass (Components|GetOwner _asbp_bullet) "/Game/CyberTanks/TankBase/Modules/BP_TankPart_Base.BP_TankPart_Base_C"
    (:False
      (bind _canuse (CallFunction|CanUse))
      (if _canuse
        (CallFunction|DamageShield (Variables|/Game/CyberTanks/TankBase/Modules/CannonModule/BP_Bullet.BP_Bullet_C|GetHPDamage _asbp_bullet) (Variables|/Game/CyberTanks/TankBase/Modules/CannonModule/BP_Bullet.BP_Bullet_C|GetEnergyDamage _asbp_bullet))
        (Actor|DestroyActor _asbp_bullet)))))

(event Custom|DamageShield
  (params (HP :type Float%20%28double-precision%29) (Energy :type Float%20%28double-precision%29))
  (Default|Damage (Variables|Default|GetAC_Energon) 0.0 HP)
  (Default|Damage (Variables|Default|GetAC_Energon) 0.0 Energy)
  (Development|PrintString "Trafiony xd"))

(event Custom|Shield_ON/OFF
  (params (On? :type Boolean))
  (if On?
    (Rendering|SetVisibility (Variables|Default|GetShield_Sphere) true false)
    (Variables|/Script/Engine.PrimitiveComponent|SetbGenerateOverlapEvents (Variables|Default|GetShield_Sphere) true)
    (else
      (Rendering|SetVisibility (Variables|Default|GetShield_Sphere) false false)
      (Variables|/Script/Engine.PrimitiveComponent|SetbGenerateOverlapEvents (Variables|Default|GetShield_Sphere) false))))

(event Custom|CustomEvent
  (Utilities|FlowControl|FlipFlop
    (:A
      (CallFunction|ShieldON/OFF true))
    (:B
      (CallFunction|ShieldON/OFF false))))

(event Custom|CustomEvent_0
  (CallFunction|ShieldON/OFF false))

(event EventBeginPlay
  (bind _ac_energon (Variables|Default|GetAC_Energon))
  (|CallParentFunction)
  (EventDispatchers|BindEventtoEnergyZero _ac_energon (delegate Custom|CustomEvent_0))
  (EventDispatchers|BindEventtoHPandEnergyZero _ac_energon (delegate Custom|CustomEvent_0))
  (EventDispatchers|BindEventtoHPZero _ac_energon (delegate Custom|CustomEvent_0))
  (EventDispatchers|BindEventtoInteractStartedEvent (delegate Custom|CustomEvent))
  (Utilities|FlowControl|Delay 0.1)
  (Transformation|SetWorldLocation (Variables|Default|GetShield_Sphere) (Transformation|GetWorldLocation (Variables|/Game/CyberTanks/TankBase/Vehicle/BP_Vehicle.BP_Vehicle_C|GetStaticMesh (Variables|Default|GetVehicleOwner))) false false)
  (CallFunction|ShieldON/OFF false))

(fn ConstructionScript
  (|CallParentFunction))