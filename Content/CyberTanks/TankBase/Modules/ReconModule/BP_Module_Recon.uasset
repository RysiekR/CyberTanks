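; BP_Module_Recon is a tank recon module that zooms the camera out while the interact input is held and energy remains.
; It extends the owning vehicle's spring arm, then restores it on release or when its Energon component's HP or energy hits zero.
; Release also charges energy proportional to hold time and uses a FlipFlop to alternately switch all top-level enemy indicator widgets off and on.
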(event HPZero(AC_Energon)
  (Development|PrintString "recon energy 0" true true "(R=1.000000,G=0.810651,B=0.000000,A=1.000000)")
  (CallFunction|ZoomBack))

(event EnergyZero(AC_Energon)
  (Development|PrintString "recon energy 0" true true "(R=1.000000,G=0.810651,B=0.000000,A=1.000000)")
  (CallFunction|ZoomBack))

(event HPandEnergyZero(AC_Energon)
  (Development|PrintString "recon energy 0" true true "(R=1.000000,G=0.810651,B=0.000000,A=1.000000)")
  (CallFunction|ZoomBack))

(event Custom|ZoomOut
  ;[0.15 0.15 0.15 0.5] Zoom
  (Variables|/Script/Engine.SpringArmComponent|SetTargetArmLength (Variables|/Game/CyberTanks/TankBase/Vehicle/BP_Vehicle.BP_Vehicle_C|GetSpringArm (Variables|Default|GetVehicleOwner)) (+ (Variables|Default|GetArmLength) (Variables|Default|GetZoomOutLength))))

(event Custom|ZoomBack
  ;[0.15 0.15 0.15 0.5] Zoom
  (Variables|/Script/Engine.SpringArmComponent|SetTargetArmLength (Variables|/Game/CyberTanks/TankBase/Vehicle/BP_Vehicle.BP_Vehicle_C|GetSpringArm (Variables|Default|GetVehicleOwner)) (Variables|Default|GetArmLength)))

(event Custom|energyzero)

(event Input|EnhancedActionEvents|EnhancedInputActionIA_Interact
  (params (ActionValue :type Boolean) (ElapsedSeconds :type Float%20%28double-precision%29) (TriggeredSeconds :type Float%20%28double-precision%29) (InputAction :type Input%20Action%20Object%20Reference :default "/Game/ThirdPerson/Input/Actions/IA_Interact.IA_Interact"))
  (bind _returnvalue (* ElapsedSeconds 5.0))
  ;[0.15 0.15 0.15 0.5] Zoom
  (:Started
    (if (> (Variables|/Game/CyberTanks/EnergonComponent/AC_Energon.AC_Energon_C|GetEnergy (Variables|Default|GetAC_Energon)) 0.0)
      (CallFunction|ZoomOut)))
  (:Completed
    (CallFunction|ZoomBack)
    (Default|Damage (Variables|Default|GetAC_Energon) 0.0 _returnvalue)
    (Development|PrintText (Utilities|Text|FormatText "used {a} energy" _returnvalue))
    (Utilities|FlowControl|FlipFlop
      (:A
        (bind _foundwidgets (Widget|GetAllWidgetsOfClass "/Game/CyberTanks/UI/WBP_EnemyIndicators.WBP_EnemyIndicators_C" true))
        (for _array_element _foundwidgets
          (Default|EventSwitchingEnemyIndicators _array_element false)))
      (:B
        (bind _foundwidgets_2 (Widget|GetAllWidgetsOfClass "/Game/CyberTanks/UI/WBP_EnemyIndicators.WBP_EnemyIndicators_C" true))
        (for _array_element_2 _foundwidgets_2
          (Default|EventSwitchingEnemyIndicators _array_element_2 true))))))

(event EventBeginPlay
  (Variables|Default|SetArmLength (Variables|/Script/Engine.SpringArmComponent|GetTargetArmLength (Variables|/Game/CyberTanks/TankBase/Vehicle/BP_Vehicle.BP_Vehicle_C|GetSpringArm (Variables|Default|GetVehicleOwner))))
  (|CallParentFunction))

(fn ConstructionScript
  (|CallParentFunction))