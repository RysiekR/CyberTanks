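; Game mode for local multiplayer CyberTanks, where player characters share a modular tank built from saved configuration.
; On BeginPlay it creates three extra local players, assigns each controller a minigame render target and material, then builds the saved tank.
; BuildTank spawns a DT_TankBaseList base with its modules and stores it in BP_MPGameInstance.
; Characters attach to its SpawnPoint; rebuilding saves and destroys other vehicles.
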(event Custom|TestPrint
  (params (module%20names :type Array%20of%20ENUM_ModuleNames%20Enums :default "NewEnumerator0") (vehicle%20name :type ENUM_VehicleBaseNames%20Enum :default "NewEnumerator0"))
  ;[0.15 0.15 0.15 0.5] Test print
  (for _array_element module%20names
    (Variables|Default|SetTestStringVar (Utilities|String|Append (Variables|Default|GetTestStringVar) (Utilities|String|EnumtoString _array_element) " 
")))
  (Development|PrintText (Utilities|Text|FormatText "Config to save: 
nunmber of parts:{a} 
vehicle base:{b} 
part names: 
{c}" (Utilities|Array|Length module%20names) (Utilities|String|EnumtoString vehicle%20name) (Utilities|Text|FormatText (Utilities|Text|ToText(String) (Variables|Default|GetTestStringVar)))) true true "(R=0.000000,G=1.000000,B=0.663957,A=1.000000)" 2e+01))

(event Custom|InitPlayers
  (Development|PrintString "init players")
  (for _index (range 1 3)
    (Class|GameplayStatics|CreatePlayer -1))
  (Variables|Default|SetDefaultPawnClass "/Game/ThirdPerson/Blueprints/BP_ThirdPersonCharacter.BP_ThirdPersonCharacter_C")
  ;[0.15 0.15 0.15 0.5] Assigning render targets for minigames to each controller
  (bind _outactors (Actor|GetAllActorsOfClass "/Game/CyberTanks/MultiPlayerSetup/PC_MPGame.PC_MPGame_C"))
  (for (_array_element _array_index) _outactors
    (Variables|/Game/CyberTanks/MultiPlayerSetup/PC_MPGame.PC_MPGame_C|SetRenderTarget _array_element (Utilities|Array|Get(acopy) (Variables|Default|GetRenderTexturesForMiniGames) _array_index))
    (Variables|/Game/CyberTanks/MultiPlayerSetup/PC_MPGame.PC_MPGame_C|SetRenderMaterial _array_element (Utilities|Array|Get(acopy) (Variables|Default|GetMaterialForRT) _array_index)))
  ;[0.15 0.15 0.15 0.5] W teorii ma zniknac myszka
  (Utilities|FlowControl|DelayUntilNextTick)
  (Variables|/Script/Engine.PlayerController|SetbShowMouseCursor (Game|GetPlayerController 0) false))

(event Custom|TransportSpecificPlayerToTank
  (params (PlayerChar :type BP%20Third%20Person%20Character%20Object%20Reference))
  (bind _asbp_mpgame_instance (Utilities|Casting|CastToBP_MPGameInstance (Game|GetGameInstance)))
  (Utilities|Array|AddUnique (Variables|/Game/CyberTanks/TankBase/Vehicle/BP_Vehicle.BP_Vehicle_C|GetPlayerChars (Variables|/Game/CyberTanks/MultiPlayerSetup/BP_MPGameInstance.BP_MPGameInstance_C|GetTank _asbp_mpgame_instance)) PlayerChar)
  (Variables|/Game/ThirdPerson/Blueprints/BP_ThirdPersonCharacter.BP_ThirdPersonCharacter_C|SetFloor PlayerChar (Variables|/Game/CyberTanks/MultiPlayerSetup/BP_MPGameInstance.BP_MPGameInstance_C|GetTank _asbp_mpgame_instance))
  (Transformation|AttachComponentToComponent PlayerChar (Variables|/Game/CyberTanks/TankBase/Vehicle/BP_Vehicle.BP_Vehicle_C|GetSpawnPoint (Variables|/Game/CyberTanks/MultiPlayerSetup/BP_MPGameInstance.BP_MPGameInstance_C|GetTank _asbp_mpgame_instance)) "None" "SnapToTarget" "SnapToTarget" "KeepRelative" true))

(event Custom|SaveAndBuildNewTank
  (params (Modules :type Array%20of%20ENUM_ModuleNames%20Enums :default "NewEnumerator0") (VehicleBase :type ENUM_VehicleBaseNames%20Enum :default "NewEnumerator0"))
  (CallFunction|TestPrint Modules VehicleBase)
  (CallFunction|BuildTank Modules VehicleBase)
  (CallFunction|TransportPlayerstoNewTank)
  (bind _asbp_mpgame_instance (Utilities|Casting|CastToBP_MPGameInstance (Game|GetGameInstance)))
  (Default|SaveGame _asbp_mpgame_instance)
  (CallFunction|DeleteOldTank))

(event Custom|BuildTank
  (params (Modules :type Array%20of%20ENUM_ModuleNames%20Enums :default "NewEnumerator0") (VehicleBase :type ENUM_VehicleBaseNames%20Enum :default "NewEnumerator0"))
  (bind _returnvalue (Utilities|GetDataTableRow "/Game/CyberTanks/TankConfiguration/DT_TankBaseList.DT_TankBaseList" (Utilities|String|StringToName (Utilities|String|EnumtoString VehicleBase)))
    (:then
      (bind _returnvalue_2 (Game|SpawnActorfromClass (.base _returnvalue) (Math|Transform|MakeTransform "0.000000,0.000000,150.000000" "0, 0, 0" "1.000000,1.000000,1.000000") "AlwaysSpawn" "MultiplyWithRoot" 0 Modules (.name _returnvalue) 0))
      (bind _asbp_mpgame_instance (Utilities|Casting|CastToBP_MPGameInstance (Game|GetGameInstance)))
      (Variables|/Game/CyberTanks/MultiPlayerSetup/BP_MPGameInstance.BP_MPGameInstance_C|SetTank _asbp_mpgame_instance _returnvalue_2))))

(event Custom|DeleteOldTank
  (bind _outactors (Actor|GetAllActorsOfClass "/Game/CyberTanks/TankBase/Vehicle/BP_Vehicle.BP_Vehicle_C"))
  (bind _asbp_mpgame_instance (Utilities|Casting|CastToBP_MPGameInstance (Game|GetGameInstance)))
  (Utilities|Array|RemoveItem _outactors (Variables|/Game/CyberTanks/MultiPlayerSetup/BP_MPGameInstance.BP_MPGameInstance_C|GetTank _asbp_mpgame_instance))
  (Actor|DestroyActor _outactors))

(event Custom|TransportPlayersToNewTank
  (bind _asbp_mpgame_instance (Utilities|Casting|CastToBP_MPGameInstance (Game|GetGameInstance)))
  (bind _outactors (Actor|GetAllActorsOfClass "/Game/ThirdPerson/Blueprints/BP_ThirdPersonCharacter.BP_ThirdPersonCharacter_C"))
  (for _array_element _outactors
    (Variables|/Game/ThirdPerson/Blueprints/BP_ThirdPersonCharacter.BP_ThirdPersonCharacter_C|SetFloor _array_element (Variables|/Game/CyberTanks/MultiPlayerSetup/BP_MPGameInstance.BP_MPGameInstance_C|GetTank _asbp_mpgame_instance))
    (Utilities|Array|AddUnique (Variables|/Game/CyberTanks/TankBase/Vehicle/BP_Vehicle.BP_Vehicle_C|GetPlayerChars (Variables|/Game/CyberTanks/MultiPlayerSetup/BP_MPGameInstance.BP_MPGameInstance_C|GetTank _asbp_mpgame_instance)) _array_element)
    ;[1 0 0] Sprawdzic jak ma przenosic !!!!!!!!!!!!!!!!!!!!!!!!!!!!!!!!!!!!!!!!!!!!!!!!!!!!!!!!!!!!!!!!!!!!!!!!!!!!!!!!!!!!!
    (Transformation|AttachComponentToComponent _array_element (Variables|/Game/CyberTanks/TankBase/Vehicle/BP_Vehicle.BP_Vehicle_C|GetSpawnPoint (Variables|/Game/CyberTanks/MultiPlayerSetup/BP_MPGameInstance.BP_MPGameInstance_C|GetTank _asbp_mpgame_instance)) "None" "SnapToTarget" "SnapToTarget" "KeepRelative" true)))

(event EventBeginPlay
  ;[0.15 0.15 0.15 0.5] GameMode Init
  (CallFunction|InitPlayers)
  (bind _asbp_mpgame_instance (Utilities|Casting|CastToBP_MPGameInstance (Game|GetGameInstance)))
  (if (Variables|/Game/CyberTanks/MultiPlayerSetup/BP_MPGameInstance.BP_MPGameInstance_C|GetSaveLoaded _asbp_mpgame_instance)
    (Development|PrintString "Hello")
    (CallFunction|BuildTank (Variables|/Game/CyberTanks/MultiPlayerSetup/BP_SaveGame.BP_SaveGame_C|GetModuleNames (Variables|/Game/CyberTanks/MultiPlayerSetup/BP_MPGameInstance.BP_MPGameInstance_C|GetSave%20Game _asbp_mpgame_instance)) (Variables|/Game/CyberTanks/MultiPlayerSetup/BP_SaveGame.BP_SaveGame_C|GetVehicleBaseName (Variables|/Game/CyberTanks/MultiPlayerSetup/BP_MPGameInstance.BP_MPGameInstance_C|GetSave%20Game _asbp_mpgame_instance)))
    (Class|GameModeBase|RestartPlayer (Game|GetPlayerController 0))
    (CallFunction|TransportPlayerstoNewTank)
    (else
      (Development|PrintString "Save NOT loaded !!!!!!!!!!!!!!!!!!!!!!!!!!!!!!!!!!!!!!!!!!!!!!!!!!!!!!!!!!!!!!!!!!!!!!!!!!!!!!!!!!!!!!!!!!!!!!!!!!!!!!!!!!!!!!!!!!!!!!!!!!!!!!!!!!!!!!!!!!!!!!!!"))))

(fn ConstructionScript)