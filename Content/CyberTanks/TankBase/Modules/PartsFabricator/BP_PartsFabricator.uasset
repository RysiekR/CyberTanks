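; Tank base module that fabricates a part, currently always a repair part, once after a short delay from BeginPlay.
; ChoosePart stores the part type, and a looping timer ticks a countdown down until it clears itself and calls CreatePart.
; CreatePart spawns BP_RepairPart at PartsSpawnLocation, using the chosen type only for the actor's name.
; The choose-menu event is an empty stub.
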(event Custom|ChoosePart
  (params (Repair :type ENUM_RepairNeed%20Enum :default "NewEnumerator0"))
  (Variables|Default|SetRepair Repair))

(event Custom|CreatePart
  (Game|SpawnActorfromClass "/Game/CyberTanks/TankBase/Modules/PartsFabricator/RepairPart/BP_RepairPart.BP_RepairPart_C" (Transformation|GetWorldTransform (Variables|Default|GetPartsSpawnLocation)) "Undefined" "MultiplyWithRoot" 0 (Utilities|String|StringToName (Utilities|String|EnumtoString (Variables|Default|GetRepair))) 0))

(event Custom|OpenChooseMenu
  ;[0.15 0.15 0.15 0.5] Create widget
)

(event Custom|StartTimerForPart
  (params (CountdownTime :type Float%20%28double-precision%29))
  ;[0.15 0.15 0.15 0.5] Part creation timer
  (Variables|Default|SetCountdownTime CountdownTime)
  (bind _returnvalue (Utilities|Time|SetTimerbyEvent (delegate Custom|Countdown) (Math|Float|MakeLiteralFloat 0.1) true))
  (Variables|Default|SetCountdownHandler _returnvalue))

(event Custom|Countdown
  ;[0.15 0.15 0.15 0.5] Part creation timer
  (bind _output_get (Variables|Default|SetCountdownTime (- (Variables|Default|GetCountdownTime) (Math|Float|MakeLiteralFloat 0.1))))
  (if (<= _output_get 0.0)
    (Utilities|Time|ClearandInvalidateTimerbyHandle (Variables|Default|GetCountdownHandler))
    (CallFunction|CreatePart)))

(event EventBeginPlay
  (CallFunction|ChoosePart "NewEnumerator2")
  (CallFunction|StartTimerforPart 2.0))

(fn ConstructionScript)